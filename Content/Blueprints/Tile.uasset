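; A clickable soil tile that plays a key-sequence minigame to plant a GrowingThing_Drill, with a random soil material picked at construction.
; Clicking an empty tile takes over the view from CameraOnAStick and outlines the block via custom depth; an occupied tile forwards focus to its GrowingThing.
; Key presses are checked against Sequence, updating the prompt, tool sprite and sounds.
; Completion restores the camera and spawns the plant through the ChildActor component.
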(event OnClicked(BlockMesh)
  (params (TouchedComponent :type Primitive%20Component%20Object%20Reference))
  (bind _outactors (Actor|GetAllActorsOfClass "/Game/Blueprints/CameraOnAStick.CameraOnAStick_C"))
  (if (not (Variables|/Game/Blueprints/CameraOnAStick.CameraOnAStick_C|GetFocussing (Utilities|Array|Get(acopy) _outactors)))
    (if (== (Variables|/Script/Engine.ChildActorComponent|GetChildActorClass (Variables|Default|GetChildActor)) 0)
      (CallFunction|Focus)
      (else
        (bind _asgrowing_thing (Utilities|Casting|CastToGrowingThing (Variables|/Script/Engine.ChildActorComponent|GetChildActor (Variables|Default|GetChildActor))))
        (Default|Focus _asgrowing_thing)))))

(event Input|KeyboardEvents|AnyKey
  (params (Key :type Key%20Structure :default "AnyKey"))
  (:Pressed
    (if (Variables|Default|GetInMiniGame)
      (CallFunction|RegisterKeyPress Key))))

(fn ConstructionScript
  (bind _blockmesh (Variables|Default|GetBlockMesh))
  (switch int (Math|Random|RandomInteger 4)
    (:Default
      (Rendering|Material|SetMaterial _blockmesh 0 "/Game/Materials/Soil/soil1_Mat.soil1_Mat" :!label _label))
    (:0
      (goto _label))
    (:1
      (Rendering|Material|SetMaterial _blockmesh 0 "/Game/Materials/Soil/soil1b_Mat.soil1b_Mat"))
    (:2
      (Rendering|Material|SetMaterial _blockmesh 0 "/Game/Materials/Soil/soil2_Mat.soil2_Mat"))
    (:3
      (Rendering|Material|SetMaterial _blockmesh 0 "/Game/Materials/Soil/soil3_Mat.soil3_Mat"))))

(fn Focus
  (bind _outactors (Actor|GetAllActorsOfClass "/Game/Blueprints/CameraOnAStick.CameraOnAStick_C"))
  (if (not (Variables|/Game/Blueprints/CameraOnAStick.CameraOnAStick_C|GetFocussing (Utilities|Array|Get(acopy) _outactors)))
    (Variables|/Game/Blueprints/CameraOnAStick.CameraOnAStick_C|SetFocussing (Utilities|Array|Get(acopy) _outactors) true)
    (Variables|/Game/Blueprints/CameraOnAStick.CameraOnAStick_C|SetFocussedObject (Utilities|Array|Get(acopy) _outactors) self)
    (Game|Player|SetViewTargetwithBlend (Game|GetPlayerController 0) self 0.0 "VTBlend_Linear" 0.0 false)
    (Rendering|SetRenderCustomDepth (Variables|Default|GetBlockMesh) true)
    (CallFunction|StartMiniGame "/Game/Blueprints/GrowingThing_Drill.GrowingThing_Drill_C")
    (Variables|Default|SetInMiniGame true)))

(fn StartMiniGame
  (params (TypeOfSeed :type Growing%20Thing%20Drill%20Class%20Reference))
  (Variables|Default|SetSeedToBePlanted TypeOfSeed)
  (Development|SetHiddeninGame (Variables|Default|GetMiniGameBackground) false true)
  (Input|EnableInput (Game|GetPlayerController 0))
  (bind _output_get (Variables|Default|SetRequiredKey (Utilities|Array|Get(acopy) (Utilities|String|GetCharacterArrayfromString (Variables|Default|GetSequence)) (Variables|Default|GetCorrectKeys))))
  (Rendering|Components|TextRender|SetText (Variables|Default|GetTextRender) (Utilities|Text|ToText(String) _output_get))
  (CallFunction|SetSprite))

(fn Unfocus
  (Development|SetHiddeninGame (Variables|Default|GetMiniGameBackground) true true)
  (Rendering|SetRenderCustomDepth (Variables|Default|GetBlockMesh) false)
  (bind _outactors (Actor|GetAllActorsOfClass "/Game/Blueprints/CameraOnAStick.CameraOnAStick_C"))
  (Game|Player|SetViewTargetwithBlend (Game|GetPlayerController 0) (Utilities|Array|Get(acopy) _outactors) 0.0 "VTBlend_Linear" 0.0 false)
  (Variables|/Game/Blueprints/CameraOnAStick.CameraOnAStick_C|SetFocussing (Utilities|Array|Get(acopy) _outactors) false))

(fn RegisterKeyPress
  (params (KeyPushed :type Key%20Structure :default "AnyKey"))
  (bind _returnvalue (Class|KismetInputLibrary|KeyGetDisplayName KeyPushed))
  (bind _returnvalue_2 (Utilities|String|ToString(Text) _returnvalue))
  (if (== (Utilities|String|FindSubstring _returnvalue_2 "mouse") -1)
    (if (Utilities|Enum|Equal(Enum) _returnvalue_2 (Variables|Default|GetRequiredKey))
      (Audio|PlaySound2D "/Game/Sounds/correct_238995__qubodup__beep-ping_01_01.correct_238995__qubodup__beep-ping_01_01")
      (bind _result (Math|Integer|IncrementInt (Variables|Default|GetCorrectKeys))
        (:%20%20
          (bind _output_get (Variables|Default|SetRequiredKey (Utilities|Array|Get(acopy) (Utilities|String|GetCharacterArrayfromString (Variables|Default|GetSequence)) _result)))
          (Rendering|Components|TextRender|SetText (Variables|Default|GetTextRender) (Utilities|Text|ToText(String) _output_get))
          (if (>= (Variables|Default|GetCorrectKeys) (Utilities|String|Len (Variables|Default|GetSequence)))
            (CallFunction|FinishMiniGame)
            (else
              (CallFunction|SetSprite)))))
      (else
        (Audio|PlaySound2D "/Game/Sounds/wrong_269149__heshl__inharmonic-negative-backwards-caution-sound_01.wrong_269149__heshl__inharmonic-negative-backwards-caution-sound_01")))))

(fn SetSprite
  (bind _toolsprite (Variables|Default|GetToolSprite))
  (switch string (Variables|Default|GetRequiredKey)
    (:Default
      _)
    (:W
      (Rendering|Components|Sprite|SetSprite _toolsprite "/Game/Sprites/watering_can_Sprite.watering_can_Sprite"))
    (:D
      (Rendering|Components|Sprite|SetSprite _toolsprite "/Game/Sprites/shovel_Sprite.shovel_Sprite"))
    (:S
      (Rendering|Components|Sprite|SetSprite _toolsprite "/Game/Sprites/potato_tool_Sprite.potato_tool_Sprite"))
    (:C
      (Rendering|Components|Sprite|SetSprite _toolsprite "/Game/Sprites/shovel_Sprite.shovel_Sprite")))
  (return))

(fn FinishMiniGame
  (CallFunction|Unfocus)
  (ChildActorComponent|SetChildActorClass (Variables|Default|GetChildActor) (Variables|Default|GetSeedToBePlanted))
  (Variables|Default|SetInMiniGame false))