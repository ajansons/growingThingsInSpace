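; Clickable drill that accumulates work over time, then yields seeds through the SeedManager when harvested.
; Tick either calls DoWork or counts down an upgrade, so production pauses while upgrading.
; It has three levels that set the seed tier spawned, with the top level randomly giving a level 2 or 3 seed.
; Sprite and point light colour show working, ready and upgrading states, with a sound on ready and upgrade completion.
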(event OnClicked(PaperSprite)
  (params (TouchedComponent :type Primitive%20Component%20Object%20Reference))
  (if (Variables|Default|GetReadyToHarvest)
    (CallFunction|Harvest)))

(event EventTick
  (params (DeltaSeconds :type Float%20%28single-precision%29))
  (if (Variables|Default|GetUpgrading)
    (bind _output_get (Variables|Default|SetTimeLeftToUpgrade (- (Variables|Default|GetTimeLeftToUpgrade) DeltaSeconds)))
    (if (<= _output_get 0.0)
      (CallFunction|FinishUpgradeDrill))
    (else
      (CallFunction|DoWork DeltaSeconds))))

(event EventMakeReadytoHarvest
  (Audio|PlaySound2D "/Game/Sounds/lbr_notification_268756__morrisjm__dingaling_01.lbr_notification_268756__morrisjm__dingaling_01")
  (Rendering|Components|Light|SetLightColor (Variables|Default|GetPointLight) (Variables|Default|GetReadyColour) true)
  (switch int (Variables|Default|GetLevel)
    (:0
      (Rendering|Components|Sprite|SetSprite (Variables|Default|GetPaperSprite) "/Game/Sprites/drill1_green_Sprite.drill1_green_Sprite"))
    (:1
      (Rendering|Components|Sprite|SetSprite (Variables|Default|GetPaperSprite) "/Game/Sprites/drill2_green_Sprite.drill2_green_Sprite"))
    (:2
      (Rendering|Components|Sprite|SetSprite (Variables|Default|GetPaperSprite) "/Game/Sprites/drill3_green_Sprite.drill3_green_Sprite"))))

(event EventActorBeginOverlap
  (params (OtherActor :type Actor%20Object%20Reference)))

(fn ConstructionScript
  (|CallParentFunction)
  (Rendering|Components|Light|SetLightColor (Variables|Default|GetPointLight) (Variables|Default|GetNotReadyColour) false)
  (Variables|Default|SetWorkThreshold 3.0)
  (bind _outactors (Actor|GetAllActorsOfClass "/Game/Blueprints/SeedManager.SeedManager_C"))
  (Variables|Default|SetSeedManagerRef (Utilities|Array|Get(acopy) _outactors)))

(fn Harvest
  (Variables|Default|SetWork 0.0)
  (Variables|Default|SetReadyToHarvest false)
  (Rendering|Components|Sprite|SetSprite (Variables|Default|GetPaperSprite) "/Game/Sprites/CrappyDrill.crappyDrill")
  (Rendering|Components|Light|SetLightColor (Variables|Default|GetPointLight) (Variables|Default|GetNotReadyColour) true)
  (switch int (Variables|Default|GetLevel)
    (:Default
      (Development|PrintString "SOMETHING BROKE IN YOUR DRILL IN THE HARVEST FUNCTION"))
    (:0
      (Rendering|Components|Sprite|SetSprite (Variables|Default|GetPaperSprite) "/Game/Sprites/drill1_yellow_Sprite.drill1_yellow_Sprite")
      (CallFunction|ProduceSeed :!label _label))
    (:1
      (Rendering|Components|Sprite|SetSprite (Variables|Default|GetPaperSprite) "/Game/Sprites/drill2_yellow_Sprite.drill2_yellow_Sprite")
      (goto _label))
    (:2
      (Rendering|Components|Sprite|SetSprite (Variables|Default|GetPaperSprite) "/Game/Sprites/drill3_yellow_Sprite.drill3_yellow_Sprite")
      (goto _label))))

(fn ProduceSeed
  (bind _seedmanagerref (Variables|Default|GetSeedManagerRef))
  (switch int (Variables|Default|GetLevel)
    (:0
      (Default|SpawnLevel1Seed (Variables|Default|GetSeedManagerRef)))
    (:1
      (Default|SpawnLevel2Seed (Variables|Default|GetSeedManagerRef)))
    (:2
      (switch int (Math|Random|RandomInteger 2)
        (:Default
          (Development|PrintString "AY YO., SOMETHING BROKE IN DRILL PRODUCE SEED FUNC"))
        (:0
          (Default|SpawnLevel3Seed _seedmanagerref))
        (:1
          (Default|SpawnLevel2Seed _seedmanagerref))))))

(fn FinishUpgradeDrill
  (Rendering|Components|Light|SetLightColor (Variables|Default|GetPointLight) (Variables|Default|GetNotReadyColour) true)
  (Variables|Default|SetWork 0.0)
  (Variables|Default|SetUpgrading false)
  (switch int (Variables|Default|GetLevel)
    (:0
      (Rendering|Components|Sprite|SetSprite (Variables|Default|GetPaperSprite) "/Game/Sprites/drill2_yellow_Sprite.drill2_yellow_Sprite"))
    (:1
      (Rendering|Components|Sprite|SetSprite (Variables|Default|GetPaperSprite) "/Game/Sprites/drill3_yellow_Sprite.drill3_yellow_Sprite")))
  (Math|Integer|IncrementInt (Variables|Default|GetLevel)
    (:%20%20
      (Audio|PlaySound2D "/Game/Sounds/lbr_notification_268756__morrisjm__dingaling_01.lbr_notification_268756__morrisjm__dingaling_01"))))

(fn StartUpgradeDrill
  (if (< (Variables|Default|GetLevel) 2)
    (Rendering|Components|Light|SetLightColor (Variables|Default|GetPointLight) (Variables|Default|GetUpgradingColour) true)
    (Variables|Default|SetTimeLeftToUpgrade (Variables|Default|GetUpgradeTime))
    (Variables|Default|SetUpgrading true)
    (switch int (Variables|Default|GetLevel)
      (:0
        (Rendering|Components|Sprite|SetSprite (Variables|Default|GetPaperSprite) "/Game/Sprites/drill1_red_Sprite.drill1_red_Sprite"))
      (:1
        (Rendering|Components|Sprite|SetSprite (Variables|Default|GetPaperSprite) "/Game/Sprites/drill2_red_Sprite.drill2_red_Sprite")))))