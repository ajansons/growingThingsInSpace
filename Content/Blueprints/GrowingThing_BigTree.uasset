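; Big tree growing thing that the player harvests through a key-sequence minigame.
; Tick calls DoWork; becoming ready swaps the sprite and plays a sound, and clicking the ready tree calls Focus.
; StartMiniGame shows the minigame and enables input, then non-mouse key names are matched against a random string from Chars.
; Wrong keys only play a sound, while completing the sequence resets work, restores the unripe sprite and picks a new sequence.
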(event OnClicked(PaperSprite)
  (params (TouchedComponent :type Primitive%20Component%20Object%20Reference))
  (if (Variables|Default|GetReadyToHarvest)
    (CallFunction|Focus)))

(event EventMakeReadytoHarvest
  (Rendering|Components|Sprite|SetSprite (Variables|Default|GetPaperSprite) "/Game/Sprites/big_tree_Sprite.big_tree_Sprite")
  (Audio|PlaySound2D "/Game/Sounds/lbr_notification_268756__morrisjm__dingaling_01.lbr_notification_268756__morrisjm__dingaling_01"))

(event EventBeginPlay)

(event Collision|EventActorBeginOverlap
  (params (OtherActor :type Actor%20Object%20Reference)))

(event EventTick
  (params (DeltaSeconds :type Float%20%28single-precision%29))
  (CallFunction|DoWork DeltaSeconds))

(event EventStartMiniGame
  (Development|SetHiddeninGame (Variables|Default|GetMinigameBackground) false true)
  (Input|EnableInput (Game|GetPlayerController 0))
  (Variables|Default|SetRequiredKey (Utilities|Array|Get(acopy) (Utilities|String|GetCharacterArrayfromString (Variables|Default|GetSequence)) (Variables|Default|GetCorrectKeys))))

(event Input|KeyboardEvents|AnyKey
  (params (Key :type Key%20Structure :default "AnyKey"))
  (:Pressed
    (if (Variables|Default|GetInMiniGame)
      (CallFunction|RegisterKeyPress Key))))

(fn ConstructionScript
  (bind _chars (Variables|Default|GetChars))
  (|CallParentFunction)
  (Variables|Default|SetWorkThreshold 3.0)
  (Variables|Default|SetSequence (Utilities|Array|Get(acopy) _chars (Math|Random|RandomInteger (- (Utilities|Array|Length _chars) 1)))))

(fn RegisterKeyPress
  (params (PressedKey :type Key%20Structure :default "AnyKey"))
  (bind _returnvalue (Class|KismetInputLibrary|KeyGetDisplayName PressedKey))
  (bind _chars (Variables|Default|GetChars))
  (bind _returnvalue_2 (Utilities|String|ToString(Text) _returnvalue))
  (if (== (Utilities|String|FindSubstring _returnvalue_2 "mouse") -1)
    (if (Utilities|Enum|Equal(Enum) _returnvalue_2 (Variables|Default|GetRequiredKey))
      (Audio|PlaySound2D "/Game/Sounds/correct_238995__qubodup__beep-ping_01_01.correct_238995__qubodup__beep-ping_01_01")
      (bind _result (Math|Integer|IncrementInt (Variables|Default|GetCorrectKeys))
        (:%20%20
          (Variables|Default|SetRequiredKey (Utilities|Array|Get(acopy) (Utilities|String|GetCharacterArrayfromString (Variables|Default|GetSequence)) _result))
          (if (>= (Variables|Default|GetCorrectKeys) (Utilities|String|Len (Variables|Default|GetSequence)))
            (Variables|Default|SetWork 0.0)
            (Variables|Default|SetReadyToHarvest false)
            (CallFunction|Unfocus)
            (Development|SetHiddeninGame (Variables|Default|GetMinigameBackground) true true)
            (Variables|Default|SetCorrectKeys 0)
            (Rendering|Components|Sprite|SetSprite (Variables|Default|GetPaperSprite) "/Game/Sprites/big_unripe_Sprite.big_unripe_Sprite")
            (Audio|PlaySoundatLocation "/Game/Sounds/lbr_success_235911__thegertz__notification-sound.lbr_success_235911__thegertz__notification-sound" (Transformation|GetActorLocation))
            (Variables|Default|SetSequence (Utilities|Array|Get(acopy) _chars (Math|Random|RandomInteger (- (Utilities|Array|Length _chars) 1)))))))
      (else
        (Audio|PlaySound2D "/Game/Sounds/wrong_269149__heshl__inharmonic-negative-backwards-caution-sound_01.wrong_269149__heshl__inharmonic-negative-backwards-caution-sound_01")))))