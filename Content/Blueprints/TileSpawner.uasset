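; Grid actor that spawns a square field of Tile actors at play start and tracks a score for it.
; BeginPlay turns a single loop index into row and column with modulo and division, placing tiles at even spacing from the actor's location.
; Each tile receives this actor as its owning grid, and the AddScore event increments the score and refreshes the score text.
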(event Custom|AddScore
  ;[1 1 1] Handle scoring when block is clicked
  (Variables|Default|SetScore (+ (Variables|Default|GetScore) 1)) ; Increment score
  (Rendering|Components|TextRender|SetText (Variables|Default|GetScoreText) (Utilities|String|BuildString(Integer) "" "Score: " (Variables|Default|GetScore))) ; Update text
)

(event EventBeginPlay
  (bind _size (Variables|Default|GetSize))
  (bind _size_2 (Variables|Default|GetSize))
  (bind _blockspacing (Variables|Default|GetBlockSpacing))
  ;[1 1 1] Spawn blocks
  (for _index (range 0 (- (* _size _size) 1)) ; Loop to spawn each block
    (Game|SpawnActorfromClass "/Game/Blueprints/Tile.Tile_C" (Math|Conversions|ToTransform(Vector) (+ (Math|Vector|MakeVector (* (Math|Integer|%(Integer) _index _size_2) _blockspacing) (* (/ _index _size_2) _blockspacing) 0.0) (Transformation|GetActorLocation))) "AdjustIfPossibleButDontSpawnIfColliding" 0 self 0) ; Spawn a  block
  ))

(fn ConstructionScript)