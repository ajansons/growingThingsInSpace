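; GrowingThing is an actor that grows over time until ready to harvest and can host a minigame.
; Tick accumulates Work up to WorkThreshold, pausing while CameraOnAStick shows instructions, then sets ReadyToHarvest and calls MakeReadyToHarvest.
; Focus claims the camera's Focussing flag, switches the view to itself and starts the minigame; Unfocus delegates to RefToParentTile.
; MakeReadyToHarvest and StartMiniGame are empty hooks.
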(event EventActorBeginOverlap
  (params (OtherActor :type Actor%20Object%20Reference)))

(event EventTick
  (params (DeltaSeconds :type Float%20%28single-precision%29))
  (CallFunction|DoWork DeltaSeconds))

(fn ConstructionScript
  (bind _outactors (Actor|GetAllActorsOfClass "/Game/Blueprints/CameraOnAStick.CameraOnAStick_C"))
  (Variables|Default|SetCameraOnAStick (Utilities|Array|Get(acopy) _outactors)))

(fn Focus
  (bind _outactors (Actor|GetAllActorsOfClass "/Game/Blueprints/CameraOnAStick.CameraOnAStick_C"))
  (if (not (Variables|/Game/Blueprints/CameraOnAStick.CameraOnAStick_C|GetFocussing (Utilities|Array|Get(acopy) _outactors)))
    (Variables|/Game/Blueprints/CameraOnAStick.CameraOnAStick_C|SetFocussing (Utilities|Array|Get(acopy) _outactors) true)
    (Game|Player|SetViewTargetwithBlend (Game|GetPlayerController 0) self 0.0 "VTBlend_Linear" 0.0 false)
    (Variables|Default|SetInMiniGame true)
    (CallFunction|StartMiniGame)))

(fn MakeReadytoHarvest)

(fn StartMiniGame)

(fn Unfocus
  (Variables|Default|SetInMiniGame false)
  (Default|Unfocus (Variables|Default|GetRefToParentTile)))

(fn DoWork
  (params (DeltaTime :type Float%20%28single-precision%29))
  (if (not (or (Variables|/Game/Blueprints/CameraOnAStick.CameraOnAStick_C|GetReadingInstructions (Variables|Default|GetCameraOnAStick)) (Variables|Default|GetReadyToHarvest)))
    (bind _output_get (Variables|Default|SetWork (+ DeltaTime (Variables|Default|GetWork))))
    (if (> _output_get (Variables|Default|GetWorkThreshold))
      (Variables|Default|SetReadyToHarvest true)
      (CallFunction|MakeReadytoHarvest))))