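; A growable Venus flytrap that is harvested through a typing mini-game.
; Tick feeds work through DoWork; once ready, the plant changes sprite, chimes and can be clicked to focus.
; In the mini-game, key presses count only while the timed jaw is open and must match the next character of Sequence.
; Completing the sequence resets work, unfocuses and returns the plant to unripe, with sounds for right, wrong and success.
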(event OnClicked(PaperSprite)
  (params (TouchedComponent :type Primitive%20Component%20Object%20Reference))
  (if (Variables|Default|GetReadyToHarvest)
    (CallFunction|Focus)))

(event EventMakeReadytoHarvest
  (Rendering|Components|Sprite|SetSprite (Variables|Default|GetPaperSprite) "/Game/Sprites/venus_Sprite.venus_Sprite")
  (Audio|PlaySound2D "/Game/Sounds/lbr_notification_268756__morrisjm__dingaling_01.lbr_notification_268756__morrisjm__dingaling_01"))

(event EventBeginPlay)

(event Collision|EventActorBeginOverlap
  (params (OtherActor :type Actor%20Object%20Reference)))

(event EventTick
  (params (DeltaSeconds :type Float%20%28single-precision%29))
  (CallFunction|DoWork DeltaSeconds)
  (if (Variables|Default|GetInMiniGame)
    (if (Variables|Default|GetJawOpen?)
      (bind _output_get (Variables|Default|SetTimeLeftOnJaw (- (Variables|Default|GetTimeLeftOnJaw) DeltaSeconds)))
      (if (<= _output_get 0.0)
        (Variables|Default|SetJawOpen? false)
        (Rendering|Components|Sprite|SetSprite (Variables|Default|GetPaperSprite2) "/Game/Sprites/jaw_closed_Sprite.jaw_closed_Sprite")))))

(event EventStartMiniGame
  (Development|SetHiddeninGame (Variables|Default|GetMinigameBackground) false true)
  (Input|EnableInput (Game|GetPlayerController 0))
  (bind _output_get (Variables|Default|SetRequiredKey (Utilities|Array|Get(acopy) (Utilities|String|GetCharacterArrayfromString (Variables|Default|GetSequence)) (Variables|Default|GetCorrectKeys))))
  (Rendering|Components|TextRender|SetText (Variables|Default|GetTextRender) (Utilities|Text|ToText(String) _output_get)))

(event Input|KeyboardEvents|AnyKey
  (params (Key :type Key%20Structure :default "AnyKey"))
  (:Pressed
    (if (Variables|Default|GetInMiniGame)
      (if (Variables|Default|GetJawOpen?)
        (CallFunction|RegisterKeyPress Key)))))

(fn ConstructionScript
  (|CallParentFunction)
  (Variables|Default|SetWorkThreshold 3.0))

(fn RegisterKeyPress
  (params (PressedKey :type Key%20Structure :default "AnyKey"))
  (bind _returnvalue (Class|KismetInputLibrary|KeyGetDisplayName PressedKey))
  (bind _returnvalue_2 (Utilities|String|ToString(Text) _returnvalue))
  (if (== (Utilities|String|FindSubstring _returnvalue_2 "mouse") -1)
    (if (Utilities|Enum|Equal(Enum) _returnvalue_2 (Variables|Default|GetRequiredKey))
      (Audio|PlaySound2D "/Game/Sounds/correct_238995__qubodup__beep-ping_01_01.correct_238995__qubodup__beep-ping_01_01")
      (bind _result (Math|Integer|IncrementInt (Variables|Default|GetCorrectKeys))
        (:%20%20
          (bind _output_get (Variables|Default|SetRequiredKey (Utilities|Array|Get(acopy) (Utilities|String|GetCharacterArrayfromString (Variables|Default|GetSequence)) _result)))
          (Rendering|Components|TextRender|SetText (Variables|Default|GetTextRender) (Utilities|Text|ToText(String) _output_get))
          (if (>= (Variables|Default|GetCorrectKeys) (Utilities|String|Len (Variables|Default|GetSequence)))
            (Variables|Default|SetWork 0.0)
            (Variables|Default|SetReadyToHarvest false)
            (CallFunction|Unfocus)
            (Development|SetHiddeninGame (Variables|Default|GetMinigameBackground) true true)
            (Variables|Default|SetCorrectKeys 0)
            (Rendering|Components|Sprite|SetSprite (Variables|Default|GetPaperSprite) "/Game/Sprites/venus_unripe_Sprite.venus_unripe_Sprite")
            (Audio|PlaySoundatLocation "/Game/Sounds/lbr_success_235911__thegertz__notification-sound.lbr_success_235911__thegertz__notification-sound" (Transformation|GetActorLocation)))))
      (else
        (Audio|PlaySound2D "/Game/Sounds/wrong_269149__heshl__inharmonic-negative-backwards-caution-sound_01.wrong_269149__heshl__inharmonic-negative-backwards-caution-sound_01")))))